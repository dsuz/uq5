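; BP_GASActor is an actor that exercises the Gameplay Ability System through debug keys.
; On BeginPlay it grants GA_1 and GA_2 to its AbilitySystem component.
; Keys 1 and 2 both try to activate abilities by the same Test tag.
; Key 3 calls RemoveGameplayTags on all owned tags, and key 4 prints each owned tag's name.
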(event `self.ReceiveBeginPlay`
  (bind _abilitysystem (`self.AbilitySystem`))
  (`AbilitySystemComponent.K2_GiveAbility` _abilitysystem "/Game/GA_1.GA_1_C" 0 -1)
  (`AbilitySystemComponent.K2_GiveAbility` _abilitysystem "/Game/GA_2.GA_2_C" 0 -1))

(event `Key|One`
  (params (Key :type "Key Structure"))
  (:`Pressed`
    (`AbilitySystemComponent.TryActivateAbilitiesByTag` (`self.AbilitySystem`) (`BlueprintGameplayTagLibrary.MakeLiteralGameplayTagContainer` (struct :`GameplayTags` (struct :`(TagName` "Test")))) true)))

(event `Key|Two`
  (params (Key :type "Key Structure"))
  (:`Pressed`
    (`AbilitySystemComponent.TryActivateAbilitiesByTag` (`self.AbilitySystem`) (`BlueprintGameplayTagLibrary.MakeLiteralGameplayTagContainer` (struct :`GameplayTags` (struct :`(TagName` "Test")))) true)))

(event `Key|Three`
  (params (Key :type "Key Structure"))
  (:`Pressed`
    (`AbilitySystemBlueprintLibrary.RemoveGameplayTags` self (`BlueprintGameplayTagLibrary.GetOwnedGameplayTags` (`self.AbilitySystem`)))))

(event `Key|Four`
  (params (Key :type "Key Structure"))
  (:`Pressed`
    (for _array_element (`BlueprintGameplayTagLibrary.BreakGameplayTagContainer` (`BlueprintGameplayTagLibrary.GetOwnedGameplayTags` (`self.AbilitySystem`)))
      (`KismetSystemLibrary.PrintString` (`KismetStringLibrary.Conv_NameToString` (`BlueprintGameplayTagLibrary.GetTagName` _array_element))))))

(fn `UserConstructionScript`)