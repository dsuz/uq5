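; BP_EnemyController is the enemy AI controller that drives enemies through the BT_Enemy behavior tree.
; On BeginPlay it initializes the BBEnemy blackboard, storing the player pawn as the chase target along with a wait time, set only if that pawn is valid.
; It then copies its walk speed, run speed and walk range variables into blackboard keys before running the tree.
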(event `self.ReceiveBeginPlay`
  (bind _returnvalue (`GameplayStatics.GetPlayerPawn` 0))
  (`|ExecutionSequence`
    (:`then_0`
      ; BlackBoard を取得する
      (bind _blackboardcomponent (`self.UseBlackboard` (`self.BBEnemy`)))
      (set `self.BBComp` _blackboardcomponent))
    (:`then_1`
      ;[1 1 1] BlackBoard に値を設定する
      (`/Engine/EditorBlueprintResources/StandardMacros.IsValid` _returnvalue
        (:`Is Valid`
          (`BlackboardComponent.SetValueAsObject` (`self.BBComp`) "ChaseActorKey" _returnvalue)
          (`BlackboardComponent.SetValueAsFloat` (`self.BBComp`) "WaitTimeKey" (`self.WaitTime`)))))
    (:`then_2`
      (`BlackboardComponent.SetValueAsFloat` (`self.BBComp`) "WalkSpeedKey" (`self.WalkSpeed`))
      (`BlackboardComponent.SetValueAsFloat` (`self.BBComp`) "RunSpeedKey" (`self.RunSpeed`))
      (`BlackboardComponent.SetValueAsFloat` (`self.BBComp`) "WalkRangeKey" (`self.WalkRange`)))
    (:`then_3`
      ;[1 1 1] ビヘイビアツリーを実行
      (`self.RunBehaviorTree` "/Game/UnrealQuest5/AI/BT_Enemy.BT_Enemy"))))

(fn `UserConstructionScript`)