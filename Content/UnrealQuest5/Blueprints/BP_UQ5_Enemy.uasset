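; Enemy character for UnrealQuest5 that can attack, take hits and die.
; The Attack event only plays an attack montage, with no caller or damage logic in this Blueprint.
; BeginPlay binds the any-damage delegate; each hit prints the causer and removes one Life, regardless of damage amount.
; At zero Life, Die disables movement, turns the mesh into a ragdoll launched upward from the pelvis, then destroys it after a short lifespan.
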(event `Attack`
  ;[1 0 0 0.5] 攻撃
  (`|PlayMontage` (`self.Mesh`) "/Game/UnrealQuest5/Characters/Mannequins/Animations/UQ5/AM_Enemy_Attack01.AM_Enemy_Attack01"))

(event `self.ReceiveBeginPlay`
  (add `self.OnTakeAnyDamage` (`|CreateDelegate` :!event `Damaged`)))

(event `Damaged` :!signature `self.OnTakeAnyDamage`
  (params (DamagedActor :type "Actor Object Reference") (Damage :type "Float (single-precision)") (DamageType :type "DamageType Object Reference") (InstigatedBy :type "Controller Object Reference") (DamageCauser :type "Actor Object Reference"))
  (bind _life (`self.Life`))
  ; ダメージを与える
  (`KismetSystemLibrary.PrintString` (`KismetStringLibrary.Concat_StrStr` "Damage Caused by: " (`KismetSystemLibrary.GetDisplayName` DamageCauser)))
  (`/Engine/EditorBlueprintResources/StandardMacros.DecrementInt` _life
    (:`  `
      (if (<= _life 0)
        (`self.Die` DamageCauser)))))

(event `Die`
  (params (`Damage Causer` :type "Actor Object Reference"))
  (bind _mesh (`self.Mesh`))
  ; 死亡演出
  (`CharacterMovementComponent.DisableMovement` (`self.CharacterMovement`))
  (`PrimitiveComponent.SetCollisionProfileName` _mesh "Ragdoll" true)
  (`PrimitiveComponent.SetSimulatePhysics` _mesh true)
  (`PrimitiveComponent.AddImpulse` _mesh (0.0 0.0 4000.0) "pelvis" true) ; 吹っ飛ばす
  (`self.SetLifeSpan` 5.0))

(fn `UserConstructionScript`)